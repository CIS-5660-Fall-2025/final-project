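; Level manager actor that builds a continuous strip of terrain by spawning BP_TerrainPiece actors along +X.
; Spawning starts on BeginPlay and repeats on a looping timer, independent of player progress.
; The first piece sits beneath the player, and each later one is offset from the previous piece by its dynamic mesh's bounding-box X length.
; Pieces accumulate in the TerrainPieces array and are never removed here.
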(event `self.ReceiveBeginPlay`
  (set `self.Player Ref` (`GameplayStatics.GetPlayerCharacter` 0))
  (`self.Spawn Terrain`)
  (`KismetSystemLibrary.K2_SetTimer` null "Spawn Terrain" 0.6 true))

(fn `Spawn Terrain`
  (locals (`Spawn Location` :type "Vector Structure"))
  (bind _player_ref (`self.Player Ref`))
  (bind _terrain_pieces (`self.Terrain Pieces`))
  (bind _dynamic_mesh_component (`/Game/LevelActors/BP_TerrainPiece.Dynamic Mesh Component` (`|GetArrayItem` _terrain_pieces (- (`KismetArrayLibrary.Array_Length` _terrain_pieces) 1))))
  (`|ExecutionSequence`
    (:`then_0`
      (if (== (`KismetArrayLibrary.Array_Length` (`self.Terrain Pieces`)) 0)
        (set `local.Spawn Location` (- (`self.K2_GetActorLocation` _player_ref) (`KismetMathLibrary.MakeVector` 0.0 0.0 (`CapsuleComponent.GetScaledCapsuleHalfHeight` (`Character.CapsuleComponent` _player_ref))) (0.0 0.0 300.0)))
        (else
          (bind _returnvalue (`BaseDynamicMeshComponent.GetDynamicMesh` _dynamic_mesh_component))
          (bind (_min _max) (break `Box` (`GeometryScriptLibrary_MeshQueryFunctions.GetMeshBoundingBox` _returnvalue)))
          (set `local.Spawn Location` (+ (`KismetMathLibrary.MakeVector` (* (- (.x _min) (.x _max)) -1.0)) (`SceneComponent.K2_GetComponentLocation` _dynamic_mesh_component))))))
    (:`then_1`
      (bind _returnvalue_2 (`|SpawnActorFromClass` "/Game/LevelActors/BP_TerrainPiece.BP_TerrainPiece_C" (`KismetMathLibrary.MakeTransform` (`local.Spawn Location`)) "Undefined" "MultiplyWithRoot" null null))
      (`KismetArrayLibrary.Array_Add` (`self.Terrain Pieces`) _returnvalue_2))))

(fn `UserConstructionScript`)