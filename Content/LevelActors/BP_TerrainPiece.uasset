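; BP_TerrainPiece is a short-lived terrain slab actor with a music-responsive material, destroying itself after TimeToLive.
; Its construction script appends a box to a dynamic mesh and generates simple collision from it, then calls a boolean subtract with no tool mesh shown.
; On BeginPlay it creates a dynamic instance of M_MusicResponse and feeds it the BPM read from the CharacterBase actor.
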(event `self.ReceiveBeginPlay`
  (`KismetSystemLibrary.K2_SetTimerDelegate` (delegate `Destroy Self`) (`self.Time to Live`))
  (`self.Set Up Material`))

(event `Destroy Self`
  (`self.K2_DestroyActor`))

(event `self.ReceiveActorBeginOverlap`
  (params (OtherActor :type "Actor Object Reference")))

(fn `Set Up Material`
  (bind _dynamic_mesh_component (`self.Dynamic Mesh Component`))
  (bind _returnvalue (`PrimitiveComponent.CreateDynamicMaterialInstance` _dynamic_mesh_component 0 "/Game/Materials/M_MusicResponse.M_MusicResponse" "None"))
  (bind _returnvalue_2 (`GameplayStatics.GetActorOfClass` "/Script/MusicGame.CharacterBase"))
  (`MaterialInstanceDynamic.SetScalarParameterValue` _returnvalue "BPM" (`CharacterBase.bpm` _returnvalue_2))
  (`PrimitiveComponent.SetMaterial` _dynamic_mesh_component 0 _returnvalue))

(fn `UserConstructionScript`
  (bind _returnvalue (`BaseDynamicMeshComponent.GetDynamicMesh` (`self.Dynamic Mesh Component`)))
  (bind _output_get (set `self.Dynamic Mesh` _returnvalue))
  (bind _returnvalue_2 (`GeometryScriptLibrary_MeshPrimitiveFunctions.AppendBox` _output_get (struct) (struct) 400.0 1200.0 20.0 0 0 0 "Base" null))
  (bind _returnvalue_3 (`GeometryScriptLibrary_CollisionFunctions.GenerateCollisionFromMesh` _returnvalue_2 (struct) null))
  (`GeometryScriptLibrary_CollisionFunctions.SetSimpleCollisionOfDynamicMeshComponent` _returnvalue_3 (`self.Dynamic Mesh Component`) (struct) null)
  (`GeometryScriptLibrary_MeshBooleanFunctions.ApplyMeshBoolean` (`self.Dynamic Mesh`) (struct) null (struct) "Subtract" (struct) null))