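; Grid-based werewolf enemy that chases the Wizard one tile per step and checks for player death after moving.
; AI_MoveOneStepTowardsWizard counts down stuns or pathfinds, switching tile mappings during DestroyPhase, then calls a directional move event.
; Move events enter Ground or Bridge tiles, or flatten Trees in DestroyPhase, using timeline lerps, AnimBP flags and a Wizard movement lock.
; Instant-move WerewolfUp/Down/Left/Right variants are only called from never-run nodes.
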(event `self.ReceiveBeginPlay`
  (bind _outactors (`GameplayStatics.GetAllActorsOfClass` "/MegaGrid/Blueprints/Core/BP_GridManager.BP_GridManager_C"))
  (set `self.Grid Manager` (`|GetArrayItem` _outactors))
  (bind _outactors_2 (`GameplayStatics.GetAllActorsOfClassWithTag` "/Game/LevelPrototyping/BP_LevelGlobals.BP_LevelGlobals_C" "LevelGlobals"))
  (set `self.Global Var` (`|GetArrayItem` _outactors_2))
  (bind _returnvalue (`GridUtils.GetIndexFromLocation` (`self.K2_GetActorLocation`)))
  (set `self.Current Cord` _returnvalue)
  (bind _outactors_3 (`GameplayStatics.GetAllActorsOfClass` "/Game/BattleWizardPBR/CharacterBP/BP_Wizard.BP_Wizard_C"))
  (set `self.WizardRef` (`|GetArrayItem` _outactors_3))
  (bind _asabp_werewolf (cast `/Game/Werewolf/Animation/ABP_Werewolf` (`SkeletalMeshComponent.GetAnimInstance` (`self.Mesh`))))
  (set `self.ActionBPRef` _asabp_werewolf))

(event `EventMoveLeft`
  (bind _returnvalue (`self.K2_GetActorLocation`))
  (bind _actionbpref (`self.ActionBPRef`))
  (bind _returnvalue_2 (+ (`self.Current Cord`) (`KismetMathLibrary.Conv_Vector2DToIntPoint` (`KismetMathLibrary.MakeVector2D` 0.0 -1.0))))
  ; IA_MoveLeft
  (set `/Game/BattleWizardPBR/CharacterBP/BP_Wizard.CanMove` false (`self.WizardRef`))
  (bind _returnvalue_3 (`GridManager.GetTileData` (`self.Grid Manager`) _returnvalue_2))
  (switch `name` (`.TileType` (break `TileData` _returnvalue_3))
    (:`Ground`
      (if true :!label _label
        (`self.RotateToTarget` _returnvalue_2)
        (set `self.Current Cord` _returnvalue_2)
        (set `self.MoveStart` _returnvalue :!label _label_2)
        (set `self.MoveTarget` (`KismetMathLibrary.MakeVector` (.x _returnvalue) (`KismetMathLibrary.FClamp` (`KismetMathLibrary.Conv_IntToDouble` (+ (.y _returnvalue) -500)) -1760.0 1740.0) (.z _returnvalue)))
        (set `/Game/Werewolf/Animation/ABP_Werewolf.GroundSpeed` 2000.0 _actionbpref)
        (bind (_direction _alpha) (`Timeline|Timeline_2` :!via `PlayFromStart`)
          (:`Update`
            (`self.K2_SetActorLocation` (`KismetMathLibrary.VLerp` (`self.MoveStart`) (`self.MoveTarget`) _alpha)))
          (:`Finished`
            (set `/Game/Werewolf/Animation/ABP_Werewolf.GroundSpeed` 0.0 _actionbpref)
            (set `/Game/BattleWizardPBR/CharacterBP/BP_Wizard.CanMove` true (`self.WizardRef`))
            (set `/Game/Werewolf/Animation/ABP_Werewolf.Destroying` false (`self.ActionBPRef`))
            (`/Game/LevelPrototyping/BP_LevelGlobals.CheckPlayerDeathByMonster` (`self.Global Var`))))))
    (:`Bridge`
      (goto _label))
    (:`Tree`
      (if (`/Game/LevelPrototyping/BP_LevelGlobals.DestroyPhase` (`self.Global Var`))
        (bind _output_get (set `self.Current Cord` _returnvalue_2))
        (`GridManager.SetTileType` (`self.Grid Manager`) _output_get "Ground" "Auto" true)
        (set `/Game/Werewolf/Animation/ABP_Werewolf.Destroying` true (`self.ActionBPRef`))
        (goto _label_2)))))

(event `EventMoveUp`
  (bind _returnvalue (`self.K2_GetActorLocation`))
  (bind _actionbpref (`self.ActionBPRef`))
  (bind _returnvalue_2 (+ (`self.Current Cord`) (`KismetMathLibrary.Conv_Vector2DToIntPoint` (`KismetMathLibrary.MakeVector2D` 1.0))))
  ; IA_MoveUp
  (set `/Game/BattleWizardPBR/CharacterBP/BP_Wizard.CanMove` false (`self.WizardRef`))
  (bind _returnvalue_3 (`GridManager.GetTileData` (`self.Grid Manager`) _returnvalue_2))
  (switch `name` (`.TileType` (break `TileData` _returnvalue_3))
    (:`Ground`
      (if true :!label _label_3
        (`self.RotateToTarget` _returnvalue_2)
        (set `self.Current Cord` _returnvalue_2)
        (set `self.MoveStart` _returnvalue :!label _label_4)
        (set `self.MoveTarget` (`KismetMathLibrary.MakeVector` (`KismetMathLibrary.FClamp` (`KismetMathLibrary.Conv_IntToDouble` (+ (.x _returnvalue) 500)) -1760.0 1740.0) (.y _returnvalue) (.z _returnvalue)))
        (set `/Game/Werewolf/Animation/ABP_Werewolf.GroundSpeed` 2000.0 _actionbpref)
        (bind (_direction _alpha) (`Timeline|Timeline` :!via `PlayFromStart`)
          (:`Update`
            (`self.K2_SetActorLocation` (`KismetMathLibrary.VLerp` (`self.MoveStart`) (`self.MoveTarget`) _alpha)))
          (:`Finished`
            (set `/Game/Werewolf/Animation/ABP_Werewolf.GroundSpeed` 0.0 _actionbpref)
            (set `/Game/BattleWizardPBR/CharacterBP/BP_Wizard.CanMove` true (`self.WizardRef`))
            (set `/Game/Werewolf/Animation/ABP_Werewolf.Destroying` false (`self.ActionBPRef`))
            (`/Game/LevelPrototyping/BP_LevelGlobals.CheckPlayerDeathByMonster` (`self.Global Var`))))))
    (:`Bridge`
      (goto _label_3))
    (:`Tree`
      (if (`/Game/LevelPrototyping/BP_LevelGlobals.DestroyPhase` (`self.Global Var`))
        (bind _output_get (set `self.Current Cord` _returnvalue_2))
        (`GridManager.SetTileType` (`self.Grid Manager`) _output_get "Ground" "Auto" true)
        (set `/Game/Werewolf/Animation/ABP_Werewolf.Destroying` true (`self.ActionBPRef`))
        (goto _label_4)))))

(event `EventMoveDown`
  (bind _returnvalue (`self.K2_GetActorLocation`))
  (bind _actionbpref (`self.ActionBPRef`))
  (bind _returnvalue_2 (+ (`self.Current Cord`) (`KismetMathLibrary.Conv_Vector2DToIntPoint` (`KismetMathLibrary.MakeVector2D` -1.0))))
  ; IA_MoveDown
  (set `/Game/BattleWizardPBR/CharacterBP/BP_Wizard.CanMove` false (`self.WizardRef`))
  (bind _returnvalue_3 (`GridManager.GetTileData` (`self.Grid Manager`) _returnvalue_2))
  (switch `name` (`.TileType` (break `TileData` _returnvalue_3))
    (:`Ground`
      (if true :!label _label_5
        (`self.RotateToTarget` _returnvalue_2)
        (set `self.Current Cord` _returnvalue_2)
        (set `self.MoveStart` _returnvalue :!label _label_6)
        (set `self.MoveTarget` (`KismetMathLibrary.MakeVector` (`KismetMathLibrary.FClamp` (`KismetMathLibrary.Conv_IntToDouble` (+ (.x _returnvalue) -500)) -1760.0 1740.0) (.y _returnvalue) (.z _returnvalue)))
        (set `/Game/Werewolf/Animation/ABP_Werewolf.GroundSpeed` 2000.0 _actionbpref)
        (bind (_direction _alpha) (`Timeline|Timeline_0` :!via `PlayFromStart`)
          (:`Update`
            (`self.K2_SetActorLocation` (`KismetMathLibrary.VLerp` (`self.MoveStart`) (`self.MoveTarget`) _alpha)))
          (:`Finished`
            (set `/Game/Werewolf/Animation/ABP_Werewolf.GroundSpeed` 0.0 _actionbpref)
            (set `/Game/BattleWizardPBR/CharacterBP/BP_Wizard.CanMove` true (`self.WizardRef`))
            (set `/Game/Werewolf/Animation/ABP_Werewolf.Destroying` false (`self.ActionBPRef`))
            (`/Game/LevelPrototyping/BP_LevelGlobals.CheckPlayerDeathByMonster` (`self.Global Var`))))))
    (:`Bridge`
      (goto _label_5))
    (:`Tree`
      (if (`/Game/LevelPrototyping/BP_LevelGlobals.DestroyPhase` (`self.Global Var`))
        (bind _output_get (set `self.Current Cord` _returnvalue_2))
        (`GridManager.SetTileType` (`self.Grid Manager`) _output_get "Ground" "Auto" true)
        (set `/Game/Werewolf/Animation/ABP_Werewolf.Destroying` true (`self.ActionBPRef`))
        (goto _label_6)))))

(event `EventMoveRight`
  (bind _returnvalue (`self.K2_GetActorLocation`))
  (bind _actionbpref (`self.ActionBPRef`))
  (bind _returnvalue_2 (+ (`self.Current Cord`) (`KismetMathLibrary.Conv_Vector2DToIntPoint` (`KismetMathLibrary.MakeVector2D` 0.0 1.0))))
  ; IA_MoveRight
  (set `/Game/BattleWizardPBR/CharacterBP/BP_Wizard.CanMove` false (`self.WizardRef`))
  (bind _returnvalue_3 (`GridManager.GetTileData` (`self.Grid Manager`) _returnvalue_2))
  (switch `name` (`.TileType` (break `TileData` _returnvalue_3))
    (:`Ground`
      (if true :!label _label_7
        (`self.RotateToTarget` _returnvalue_2)
        (set `self.Current Cord` _returnvalue_2)
        (set `self.MoveStart` _returnvalue :!label _label_8)
        (set `self.MoveTarget` (`KismetMathLibrary.MakeVector` (.x _returnvalue) (`KismetMathLibrary.FClamp` (`KismetMathLibrary.Conv_IntToDouble` (+ (.y _returnvalue) 500)) -1760.0 1740.0) (.z _returnvalue)))
        (set `/Game/Werewolf/Animation/ABP_Werewolf.GroundSpeed` 2000.0 _actionbpref)
        (bind (_direction _alpha) (`Timeline|Timeline_1` :!via `PlayFromStart`)
          (:`Update`
            (`self.K2_SetActorLocation` (`KismetMathLibrary.VLerp` (`self.MoveStart`) (`self.MoveTarget`) _alpha)))
          (:`Finished`
            (set `/Game/Werewolf/Animation/ABP_Werewolf.GroundSpeed` 0.0 _actionbpref)
            (set `/Game/BattleWizardPBR/CharacterBP/BP_Wizard.CanMove` true (`self.WizardRef`))
            (set `/Game/Werewolf/Animation/ABP_Werewolf.Destroying` false (`self.ActionBPRef`))
            (`/Game/LevelPrototyping/BP_LevelGlobals.CheckPlayerDeathByMonster` (`self.Global Var`))))))
    (:`Bridge`
      (goto _label_7))
    (:`Tree`
      (if (`/Game/LevelPrototyping/BP_LevelGlobals.DestroyPhase` (`self.Global Var`))
        (bind _output_get (set `self.Current Cord` _returnvalue_2))
        (`GridManager.SetTileType` (`self.Grid Manager`) _output_get "Ground" "Auto" true)
        (set `/Game/Werewolf/Animation/ABP_Werewolf.Destroying` true (`self.ActionBPRef`))
        (goto _label_8)))))

(fn `AI_MoveOneStepTowardsWizard`
  (params (WizardRef :type "/Game/BattleWizardPBR/CharacterBP/BP_Wizard Object Reference"))
  (bind _pathfinding (`self.PathFinding`))
  (bind _stuncountdown (`self.StunCountdown`))
  (bind (_x _y) (break `IntPoint` (`self.Current Cord`)))
  (if (== _stuncountdown 0)
    (bind _returnvalue (`GridUtils.GetIndexFromLocation` (`self.K2_GetActorLocation` WizardRef)))
    (if (`/Game/LevelPrototyping/BP_LevelGlobals.DestroyPhase` (`self.Global Var`))
      (set `PathFindingComponent.TileTypeMapping` "/MegaGrid/Data/DT_TileTypeMappingDestroyPhase.DT_TileTypeMappingDestroyPhase" _pathfinding)
      (else
        (set `PathFindingComponent.TileTypeMapping` "/MegaGrid/Data/DT_TileTypeMapping.DT_TileTypeMapping" _pathfinding)))
    (bind _returnvalue_2 (`PathFindingComponent.FindPath` (`self.PathFinding`) (`self.Current Cord`) _returnvalue))
    (bind (_x_2 _y_2) (break `IntPoint` (`|GetArrayItem` (`.Path` (break `PathStruct` _returnvalue_2)))))
    (set `self.NextX` _x_2)
    (set `self.NextY` _y_2)
    (set `self.CurX` _x)
    (set `self.CurY` _y)
    (if (> (`self.NextY`) (`self.CurY`))
      (`self.EventMoveRight`)
      (elif (< (`self.NextY`) (`self.CurY`))
        (`self.EventMoveLeft`)
        (elif (> (`self.NextX`) (`self.CurX`))
          (`self.EventMoveUp`)
          (else
            (`self.EventMoveDown`)))))
    (else
      (bind _output_get (set `self.StunCountdown` (- _stuncountdown 1)))
      (if (== _output_get 0)
        (set `/Game/Werewolf/Animation/ABP_Werewolf.Stunned` false (`self.ActionBPRef`))))))

(fn `RotateToTarget`
  (params (`Target Position` :type "IntPoint Structure"))
  (bind (_x _y) (break `IntPoint` `Target Position`))
  (bind (_x_2 _y_2) (break `IntPoint` (`self.Current Cord`)))
  (bind _returnvalue (- _x _x_2))
  (`self.K2_SetActorRotation` (`KismetMathLibrary.MakeRotator` 0.0 0.0 (`KismetMathLibrary.SelectFloat` (`KismetMathLibrary.SelectFloat` -90.0 90.0 (== _returnvalue 1)) (`KismetMathLibrary.SelectFloat` 0.0 180.0 (== (- _y _y_2) 1)) (!= _returnvalue 0)))))

(fn `UserConstructionScript`)

(fn `WerewolfDown`
  (bind _returnvalue (+ (`self.Current Cord`) (`KismetMathLibrary.Conv_Vector2DToIntPoint` (`KismetMathLibrary.MakeVector2D` -1.0))))
  (bind _returnvalue_2 (`GridManager.GetTileData` (`self.Grid Manager`) _returnvalue))
  (switch `name` (`.TileType` (break `TileData` _returnvalue_2))
    (:`Ground`
      (if true :!label _label
        (set `self.Current Cord` _returnvalue)
        (`self.K2_SetActorLocation` (`KismetMathLibrary.MakeVector` (`KismetMathLibrary.FClamp` (`KismetMathLibrary.Conv_IntToDouble` (+ (.x (`self.K2_GetActorLocation`)) -500)) -1760.0 1740.0) (.y (`self.K2_GetActorLocation`)) (.z (`self.K2_GetActorLocation`))) :!label _label_2)
        (`/Game/LevelPrototyping/BP_LevelGlobals.CheckPlayerDeathByMonster` (`self.Global Var`))))
    (:`Bridge`
      (goto _label))
    (:`Tree`
      (if (`/Game/LevelPrototyping/BP_LevelGlobals.DestroyPhase` (`self.Global Var`))
        (bind _output_get (set `self.Current Cord` _returnvalue))
        (`GridManager.SetTileType` (`self.Grid Manager`) _output_get "Ground" "Auto" true)
        (goto _label_2)))))

(fn `WerewolfLeft`
  (bind _returnvalue (+ (`self.Current Cord`) (`KismetMathLibrary.Conv_Vector2DToIntPoint` (`KismetMathLibrary.MakeVector2D` 0.0 -1.0))))
  (bind _returnvalue_2 (`GridManager.GetTileData` (`self.Grid Manager`) _returnvalue))
  (switch `name` (`.TileType` (break `TileData` _returnvalue_2))
    (:`Ground`
      (if true :!label _label
        (set `self.Current Cord` _returnvalue)
        (`self.K2_SetActorLocation` (`KismetMathLibrary.MakeVector` (.x (`self.K2_GetActorLocation`)) (`KismetMathLibrary.FClamp` (`KismetMathLibrary.Conv_IntToDouble` (+ (.y (`self.K2_GetActorLocation`)) -500)) -1760.0 1740.0) (.z (`self.K2_GetActorLocation`))) :!label _label_2)
        (`/Game/LevelPrototyping/BP_LevelGlobals.CheckPlayerDeathByMonster` (`self.Global Var`))))
    (:`Bridge`
      (goto _label))
    (:`Tree`
      (if (`/Game/LevelPrototyping/BP_LevelGlobals.DestroyPhase` (`self.Global Var`))
        (bind _output_get (set `self.Current Cord` _returnvalue))
        (`GridManager.SetTileType` (`self.Grid Manager`) _output_get "Ground" "Auto" true)
        (goto _label_2)))))

(fn `WerewolfRight`
  (bind _returnvalue (+ (`self.Current Cord`) (`KismetMathLibrary.Conv_Vector2DToIntPoint` (`KismetMathLibrary.MakeVector2D` 0.0 1.0))))
  (bind _returnvalue_2 (`GridManager.GetTileData` (`self.Grid Manager`) _returnvalue))
  (switch `name` (`.TileType` (break `TileData` _returnvalue_2))
    (:`Ground`
      (if true :!label _label
        (set `self.Current Cord` _returnvalue)
        (`self.K2_SetActorLocation` (`KismetMathLibrary.MakeVector` (.x (`self.K2_GetActorLocation`)) (`KismetMathLibrary.FClamp` (`KismetMathLibrary.Conv_IntToDouble` (+ (.y (`self.K2_GetActorLocation`)) 500)) -1760.0 1740.0) (.z (`self.K2_GetActorLocation`))) :!label _label_2)
        (`/Game/LevelPrototyping/BP_LevelGlobals.CheckPlayerDeathByMonster` (`self.Global Var`))))
    (:`Bridge`
      (goto _label))
    (:`Tree`
      (if (`/Game/LevelPrototyping/BP_LevelGlobals.DestroyPhase` (`self.Global Var`))
        (bind _output_get (set `self.Current Cord` _returnvalue))
        (`GridManager.SetTileType` (`self.Grid Manager`) _output_get "Ground" "Auto" true)
        (goto _label_2)))))

(fn `WerewolfUp`
  (bind _returnvalue (+ (`self.Current Cord`) (`KismetMathLibrary.Conv_Vector2DToIntPoint` (`KismetMathLibrary.MakeVector2D` 1.0))))
  (bind _returnvalue_2 (`GridManager.GetTileData` (`self.Grid Manager`) _returnvalue))
  (switch `name` (`.TileType` (break `TileData` _returnvalue_2))
    (:`Ground`
      (if true :!label _label
        (set `self.Current Cord` _returnvalue)
        (`self.K2_SetActorLocation` (`KismetMathLibrary.MakeVector` (`KismetMathLibrary.FClamp` (`KismetMathLibrary.Conv_IntToDouble` (+ (.x (`self.K2_GetActorLocation`)) 500)) -1760.0 1740.0) (.y (`self.K2_GetActorLocation`)) (.z (`self.K2_GetActorLocation`))) :!label _label_2)
        (`/Game/LevelPrototyping/BP_LevelGlobals.CheckPlayerDeathByMonster` (`self.Global Var`))))
    (:`Bridge`
      (goto _label))
    (:`Tree`
      (if (`/Game/LevelPrototyping/BP_LevelGlobals.DestroyPhase` (`self.Global Var`))
        (bind _output_get (set `self.Current Cord` _returnvalue))
        (`GridManager.SetTileType` (`self.Grid Manager`) _output_get "Ground" "Auto" true)
        (goto _label_2)))))