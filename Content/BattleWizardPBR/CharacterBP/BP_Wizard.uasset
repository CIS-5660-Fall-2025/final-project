(event `self.ReceiveBeginPlay`
  (bind _asplayer_controller (cast `PlayerController` (`self.GetController`)))
  (bind _returnvalue (pcsubsystem `EnhancedInputLocalPlayerSubsystem` _asplayer_controller))
  (`/Engine/EditorBlueprintResources/StandardMacros.IsValid` _returnvalue
    (:`Is Valid`
      (`EnhancedInputSubsystemInterface.AddMappingContext` _returnvalue "/Game/TopDown/Input/IMC_Default.IMC_Default" 0 (struct))
      (bind _outactors (`GameplayStatics.GetAllActorsOfClass` "/MegaGrid/Blueprints/Core/BP_GridManager.BP_GridManager_C"))
      (set `self.GridManager` (`|GetArrayItem` _outactors))
      (bind _outactors_2 (`GameplayStatics.GetAllActorsOfClassWithTag` "/Game/LevelPrototyping/BP_LevelGlobals.BP_LevelGlobals_C" "LevelGlobals"))
      (set `self.GlobalVar` (`|GetArrayItem` _outactors_2))
      (bind _returnvalue_2 (`GridUtils.GetIndexFromLocation` (`self.K2_GetActorLocation`)))
      (set `self.CurrentCord` _returnvalue_2)
      (`self.UpdateTilesNearWizard`)
      (`KismetSystemLibrary.K2_SetTimer` null "SelectTileNearWizard" 0.03 true)
      (bind _outactors_3 (`GameplayStatics.GetAllActorsOfClass` "/Game/Werewolf/BP_Werewolf.BP_Werewolf_C"))
      (set `self.WerewolfRef` (`|GetArrayItem` _outactors_3))
      (bind _outactors_4 (`GameplayStatics.GetAllActorsOfClass` "/Script/Engine.ExponentialHeightFog"))
      (set `self.FogRef` (`|GetArrayItem` _outactors_4))
      (bind _asabp_wizard (cast `/Game/BattleWizardPBR/Animations/ABP_Wizard` (`SkeletalMeshComponent.GetAnimInstance` (`self.Mesh`))))
      (set `self.ActionBPRef` _asabp_wizard))))

(event `EnhancedInput|/Game/TopDown/Input/Actions/IA_MoveLeft`
  (params (ActionValue :type Boolean) (ElapsedSeconds :type "Float (double-precision)") (TriggeredSeconds :type "Float (double-precision)") (InputAction :type "InputAction Object Reference" :default "/Game/TopDown/Input/Actions/IA_MoveLeft.IA_MoveLeft"))
  (bind _returnvalue (`self.K2_GetActorLocation`))
  (bind _actionbpref (`self.ActionBPRef`))
  (bind _returnvalue_2 (+ (`self.CurrentCord`) (`KismetMathLibrary.Conv_Vector2DToIntPoint` (`KismetMathLibrary.MakeVector2D` 0.0 -1.0))))
  ; IA_MoveLeft
  (:`Started`
    (if (`self.CanMove`)
      (set `self.CanMove` false)
      (bind _returnvalue_3 (`GridManager.GetTileData` (`self.GridManager`) _returnvalue_2))
      (switch `name` (`.TileType` (break `TileData` _returnvalue_3))
        (:`Ground`
          _)
        (:`Bridge`
          _))
      (if true
        (`self.RotateToTarget` _returnvalue_2)
        (set `self.CurrentCord` _returnvalue_2)
        (set `self.MoveStart` _returnvalue)
        (set `self.MoveTarget` (`KismetMathLibrary.MakeVector` (.x _returnvalue) (`KismetMathLibrary.FClamp` (`KismetMathLibrary.Conv_IntToDouble` (+ (.y _returnvalue) -500)) -1760.0 1740.0) (.z _returnvalue)))
        (set `/Game/BattleWizardPBR/Animations/ABP_Wizard.Ground Speed` 1000.0 _actionbpref)
        (bind (_direction _alpha) (`Timeline|Timeline_1` :!via `PlayFromStart`)
          (:`Update`
            (`self.K2_SetActorLocation` (`KismetMathLibrary.VLerp` (`self.MoveStart`) (`self.MoveTarget`) _alpha)))
          (:`Finished`
            (set `/Game/BattleWizardPBR/Animations/ABP_Wizard.Ground Speed` 0.0 _actionbpref)
            (`/Game/LevelPrototyping/BP_LevelGlobals.AdvanceTurn` (`self.GlobalVar`))
            (`self.UpdateTilesNearWizard`)
            (`GridManager.RemoveStateFromTile` (`self.GridManager`) (`self.HoveredTile`) "Selected" true true)
            (set `self.CanMove` true)))))))

(event `EnhancedInput|/Game/TopDown/Input/Actions/IA_MoveUp`
  (params (ActionValue :type Boolean) (ElapsedSeconds :type "Float (double-precision)") (TriggeredSeconds :type "Float (double-precision)") (InputAction :type "InputAction Object Reference" :default "/Game/TopDown/Input/Actions/IA_MoveUp.IA_MoveUp"))
  (bind _returnvalue (`self.K2_GetActorLocation`))
  (bind _actionbpref (`self.ActionBPRef`))
  (bind _returnvalue_2 (+ (`self.CurrentCord`) (`KismetMathLibrary.Conv_Vector2DToIntPoint` (`KismetMathLibrary.MakeVector2D` 1.0))))
  ; IA_MoveUp
  (:`Started`
    (if (`self.CanMove`)
      (set `self.CanMove` false)
      (bind _returnvalue_3 (`GridManager.GetTileData` (`self.GridManager`) _returnvalue_2))
      (switch `name` (`.TileType` (break `TileData` _returnvalue_3))
        (:`Ground`
          _)
        (:`Bridge`
          _))
      (if true
        (`self.RotateToTarget` _returnvalue_2)
        (set `self.CurrentCord` _returnvalue_2)
        (set `self.MoveStart` _returnvalue)
        (set `self.MoveTarget` (`KismetMathLibrary.MakeVector` (`KismetMathLibrary.FClamp` (`KismetMathLibrary.Conv_IntToDouble` (+ (.x _returnvalue) 500)) -1760.0 1740.0) (.y _returnvalue) (.z _returnvalue)))
        (set `/Game/BattleWizardPBR/Animations/ABP_Wizard.Ground Speed` 1000.0 _actionbpref)
        (bind (_direction _alpha) (`Timeline|Timeline` :!via `PlayFromStart`)
          (:`Update`
            (`self.K2_SetActorLocation` (`KismetMathLibrary.VLerp` (`self.MoveStart`) (`self.MoveTarget`) _alpha)))
          (:`Finished`
            (set `/Game/BattleWizardPBR/Animations/ABP_Wizard.Ground Speed` 0.0 _actionbpref)
            (`/Game/LevelPrototyping/BP_LevelGlobals.AdvanceTurn` (`self.GlobalVar`))
            (`self.UpdateTilesNearWizard`)
            (`GridManager.RemoveStateFromTile` (`self.GridManager`) (`self.HoveredTile`) "Selected" true true)
            (set `self.CanMove` true)))))))

(event `EnhancedInput|/Game/TopDown/Input/Actions/IA_MoveDown`
  (params (ActionValue :type Boolean) (ElapsedSeconds :type "Float (double-precision)") (TriggeredSeconds :type "Float (double-precision)") (InputAction :type "InputAction Object Reference" :default "/Game/TopDown/Input/Actions/IA_MoveDown.IA_MoveDown"))
  (bind _returnvalue (`self.K2_GetActorLocation`))
  (bind _actionbpref (`self.ActionBPRef`))
  (bind _returnvalue_2 (+ (`self.CurrentCord`) (`KismetMathLibrary.Conv_Vector2DToIntPoint` (`KismetMathLibrary.MakeVector2D` -1.0))))
  ; IA_MoveDown
  (:`Started`
    (if (`self.CanMove`)
      (set `self.CanMove` false)
      (bind _returnvalue_3 (`GridManager.GetTileData` (`self.GridManager`) _returnvalue_2))
      (switch `name` (`.TileType` (break `TileData` _returnvalue_3))
        (:`Ground`
          _)
        (:`Bridge`
          _))
      (if true
        (`self.RotateToTarget` _returnvalue_2)
        (set `self.CurrentCord` _returnvalue_2)
        (set `self.MoveStart` _returnvalue)
        (set `self.MoveTarget` (`KismetMathLibrary.MakeVector` (`KismetMathLibrary.FClamp` (`KismetMathLibrary.Conv_IntToDouble` (+ (.x _returnvalue) -500)) -1760.0 1740.0) (.y _returnvalue) (.z _returnvalue)))
        (set `/Game/BattleWizardPBR/Animations/ABP_Wizard.Ground Speed` 1000.0 _actionbpref)
        (bind (_direction _alpha) (`Timeline|Timeline_0` :!via `PlayFromStart`)
          (:`Update`
            (`self.K2_SetActorLocation` (`KismetMathLibrary.VLerp` (`self.MoveStart`) (`self.MoveTarget`) _alpha)))
          (:`Finished`
            (set `/Game/BattleWizardPBR/Animations/ABP_Wizard.Ground Speed` 0.0 _actionbpref)
            (`/Game/LevelPrototyping/BP_LevelGlobals.AdvanceTurn` (`self.GlobalVar`))
            (`self.UpdateTilesNearWizard`)
            (`GridManager.RemoveStateFromTile` (`self.GridManager`) (`self.HoveredTile`) "Selected" true true)
            (set `self.CanMove` true)))))))

(event `EnhancedInput|/Game/TopDown/Input/Actions/IA_MoveRight`
  (params (ActionValue :type Boolean) (ElapsedSeconds :type "Float (double-precision)") (TriggeredSeconds :type "Float (double-precision)") (InputAction :type "InputAction Object Reference" :default "/Game/TopDown/Input/Actions/IA_MoveRight.IA_MoveRight"))
  (bind _returnvalue (`self.K2_GetActorLocation`))
  (bind _actionbpref (`self.ActionBPRef`))
  (bind _returnvalue_2 (+ (`self.CurrentCord`) (`KismetMathLibrary.Conv_Vector2DToIntPoint` (`KismetMathLibrary.MakeVector2D` 0.0 1.0))))
  ; IA_MoveRight
  (:`Started`
    (if (`self.CanMove`)
      (set `self.CanMove` false)
      (bind _returnvalue_3 (`GridManager.GetTileData` (`self.GridManager`) _returnvalue_2))
      (switch `name` (`.TileType` (break `TileData` _returnvalue_3))
        (:`Ground`
          _)
        (:`Bridge`
          _))
      (if true
        (`self.RotateToTarget` _returnvalue_2)
        (set `self.CurrentCord` _returnvalue_2)
        (set `self.MoveStart` _returnvalue)
        (set `self.MoveTarget` (`KismetMathLibrary.MakeVector` (.x _returnvalue) (`KismetMathLibrary.FClamp` (`KismetMathLibrary.Conv_IntToDouble` (+ (.y _returnvalue) 500)) -1760.0 1740.0) (.z _returnvalue)))
        (set `/Game/BattleWizardPBR/Animations/ABP_Wizard.Ground Speed` 1000.0 _actionbpref)
        (bind (_direction _alpha) (`Timeline|Timeline_2` :!via `PlayFromStart`)
          (:`Update`
            (`self.K2_SetActorLocation` (`KismetMathLibrary.VLerp` (`self.MoveStart`) (`self.MoveTarget`) _alpha)))
          (:`Finished`
            (set `/Game/BattleWizardPBR/Animations/ABP_Wizard.Ground Speed` 0.0 _actionbpref)
            (`/Game/LevelPrototyping/BP_LevelGlobals.AdvanceTurn` (`self.GlobalVar`))
            (`self.UpdateTilesNearWizard`)
            (`GridManager.RemoveStateFromTile` (`self.GridManager`) (`self.HoveredTile`) "Selected" true true)
            (set `self.CanMove` true)))))))

(event `EnhancedInput|/Game/TopDown/Input/Actions/IA_StayStill`
  (params (ActionValue :type Boolean) (ElapsedSeconds :type "Float (double-precision)") (TriggeredSeconds :type "Float (double-precision)") (InputAction :type "InputAction Object Reference" :default "/Game/TopDown/Input/Actions/IA_StayStill.IA_StayStill"))
  ; IA_StayStill
  (:`Started`
    (if (`self.CanMove`)
      (`/Game/LevelPrototyping/BP_LevelGlobals.AdvanceTurn` (`self.GlobalVar`)))))

(event `EnhancedInput|/Game/TopDown/Input/Actions/IA_Create`
  (params (ActionValue :type Boolean) (ElapsedSeconds :type "Float (double-precision)") (TriggeredSeconds :type "Float (double-precision)") (InputAction :type "InputAction Object Reference" :default "/Game/TopDown/Input/Actions/IA_Create.IA_Create"))
  (bind _gridmanager (`self.GridManager`))
  ; IA_Create
  (:`Started`
    (if (not (`self.Destroying`))
      (bind _contains (`self.ContainsPoint`))
      (if _contains
        (set `self.Creating` true)
        (set `/Game/BattleWizardPBR/Animations/ABP_Wizard.Action` "NewEnumerator1" (`self.ActionBPRef`))
        (bind _returnvalue (`WidgetLayoutLibrary.GetMousePositionOnViewport`))
        (bind _returnvalue_2 (`|CreateWidget` "/Game/BattleWizardPBR/WBP_SelectWheel.WBP_SelectWheel_C" null false _returnvalue))
        (bind _output_get (set `self.WheelRef` _returnvalue_2))
        (`UserWidget.AddToViewport` _output_get 0)
        (set `self.CanMove` false))))
  (:`Completed`
    (if (not (`self.Destroying`))
      (`/Engine/EditorBlueprintResources/StandardMacros.IsValid` (`self.WheelRef`)
        (:`Is Valid`
          (switch `int` (`/Game/BattleWizardPBR/WBP_SelectWheel.CurrentSelectionIndex` (`self.WheelRef`))
            (:`0`
              (`Widget.RemoveFromParent` (`self.WheelRef`))
              (set `self.CanMove` true)
              (set `self.Creating` false)
              (set `/Game/BattleWizardPBR/Animations/ABP_Wizard.Action` "NewEnumerator0" (`self.ActionBPRef`)))
            (:`1`
              (`Widget.RemoveFromParent` (`self.WheelRef`))
              (set `self.CanMove` true)
              (if (>= (`self.Energy`) 20)
                (bind _returnvalue_3 (`GridManager.GetAllTilesOfState` (`self.GridManager`) "Selected"))
                (if (not (`KismetArrayLibrary.Array_IsEmpty` _returnvalue_3))
                  (bind _returnvalue_4 (`GridManager.GetTileData` (`self.GridManager`) (`|GetArrayItem` _returnvalue_3)))
                  (set `/Game/LevelPrototyping/BP_LevelGlobals.DestroyPhase` false (`self.GlobalVar`))
                  (`ExponentialHeightFogComponent.SetSkyAtmosphereAmbientContributionColorScale` (`ExponentialHeightFog.Component` (`self.FogRef`)) (struct :`R` 0.597202 :`G` 1.0 :`B` 0.309469 :`A` 1.0))
                  (bind (_index _gcost _hcost _fcost _movementcost _parentindex _neighbors _tiletransform _tiletype) (break `TileData` _returnvalue_4))
                  (switch `name` _tiletype
                    (:`Ground`
                      (`GridManager.SetTileType` _gridmanager _index "Tree" "Runtime" true))
                    (:`Pit`
                      (`GridManager.SetTileType` _gridmanager _index "Ground" "Runtime" true))
                    (:`Water`
                      (`GridManager.SetTileType` _gridmanager _index "Bridge" "Runtime" true)))
                  (set `self.Energy` (- (`self.Energy`) 20))
                  (`/Game/LevelPrototyping/BP_LevelGlobals.AdvanceTurn` (`self.GlobalVar`))
                  (set `self.Creating` false)
                  (set `/Game/BattleWizardPBR/Animations/ABP_Wizard.Action` "NewEnumerator0" (`self.ActionBPRef`)))))))))))

(event `EnhancedInput|/Game/TopDown/Input/Actions/IA_ChangePhase`
  (params (ActionValue :type Boolean) (ElapsedSeconds :type "Float (double-precision)") (TriggeredSeconds :type "Float (double-precision)") (InputAction :type "InputAction Object Reference" :default "/Game/TopDown/Input/Actions/IA_ChangePhase.IA_ChangePhase"))
  (bind _globalvar (`self.GlobalVar`))
  (bind _component (`ExponentialHeightFog.Component` (`self.FogRef`)))
  ; IA_ChangePhase
  (:`Started`
    (if (`self.CanMove`)
      (if (>= (`self.Energy`) 10)
        (if (`/Game/LevelPrototyping/BP_LevelGlobals.DestroyPhase` _globalvar)
          (set `/Game/LevelPrototyping/BP_LevelGlobals.DestroyPhase` false _globalvar)
          (`ExponentialHeightFogComponent.SetSkyAtmosphereAmbientContributionColorScale` _component (struct :`R` 0.597202 :`G` 1.0 :`B` 0.309469 :`A` 1.0))
          (else
            (set `/Game/LevelPrototyping/BP_LevelGlobals.DestroyPhase` true _globalvar)
            (`ExponentialHeightFogComponent.SetSkyAtmosphereAmbientContributionColorScale` _component (struct :`R` 0.768151 :`G` 0.401978 :`B` 1.0 :`A` 1.0))))
        (set `self.Energy` (- (`self.Energy`) 10))))))

(event `EnhancedInput|/Game/TopDown/Input/Actions/IA_UpArrow`
  (params (ActionValue :type Boolean) (ElapsedSeconds :type "Float (double-precision)") (TriggeredSeconds :type "Float (double-precision)") (InputAction :type "InputAction Object Reference" :default "/Game/TopDown/Input/Actions/IA_UpArrow.IA_UpArrow"))
  ; Werewolf control for playtest purpose prior to the implementation of monster AI
)

(event `EnhancedInput|/Game/TopDown/Input/Actions/IA_DownArrow`
  (params (ActionValue :type Boolean) (ElapsedSeconds :type "Float (double-precision)") (TriggeredSeconds :type "Float (double-precision)") (InputAction :type "InputAction Object Reference" :default "/Game/TopDown/Input/Actions/IA_DownArrow.IA_DownArrow"))
  ; Werewolf control for playtest purpose prior to the implementation of monster AI
)

(event `EnhancedInput|/Game/TopDown/Input/Actions/IA_LeftArrow`
  (params (ActionValue :type Boolean) (ElapsedSeconds :type "Float (double-precision)") (TriggeredSeconds :type "Float (double-precision)") (InputAction :type "InputAction Object Reference" :default "/Game/TopDown/Input/Actions/IA_LeftArrow.IA_LeftArrow"))
  ; Werewolf control for playtest purpose prior to the implementation of monster AI
)

(event `EnhancedInput|/Game/TopDown/Input/Actions/IA_RightArrow`
  (params (ActionValue :type Boolean) (ElapsedSeconds :type "Float (double-precision)") (TriggeredSeconds :type "Float (double-precision)") (InputAction :type "InputAction Object Reference" :default "/Game/TopDown/Input/Actions/IA_RightArrow.IA_RightArrow"))
  ; Werewolf control for playtest purpose prior to the implementation of monster AI
)

(event `DrinkPotion`
  (bind _actionbpref (`self.ActionBPRef`))
  (set `/Game/BattleWizardPBR/Animations/ABP_Wizard.Action` "NewEnumerator5" _actionbpref)
  (`KismetSystemLibrary.Delay` 2.67)
  (set `/Game/BattleWizardPBR/Animations/ABP_Wizard.Action` "NewEnumerator0" _actionbpref))

(event `EnhancedInput|/Game/TopDown/Input/Actions/IA_Destroy`
  (params (ActionValue :type Boolean) (ElapsedSeconds :type "Float (double-precision)") (TriggeredSeconds :type "Float (double-precision)") (InputAction :type "InputAction Object Reference" :default "/Game/TopDown/Input/Actions/IA_Destroy.IA_Destroy"))
  (bind _werewolfref (`self.WerewolfRef`))
  (bind _gridmanager (`self.GridManager`))
  (bind _actionbpref (`/Game/Werewolf/BP_Werewolf.ActionBPRef` _werewolfref))
  ; IA_Destroy
  (:`Started`
    (if (not (`self.Creating`))
      (bind _contains (`self.ContainsPoint`))
      (if _contains
        (set `self.Destroying` true)
        (set `/Game/BattleWizardPBR/Animations/ABP_Wizard.Action` "NewEnumerator2" (`self.ActionBPRef`))
        (bind _returnvalue (`WidgetLayoutLibrary.GetMousePositionOnViewport`))
        (bind _returnvalue_2 (`|CreateWidget` "/Game/BattleWizardPBR/WBP_SelectWheel.WBP_SelectWheel_C" null true _returnvalue))
        (bind _output_get (set `self.WheelRef` _returnvalue_2))
        (`UserWidget.AddToViewport` _output_get 0)
        (set `self.CanMove` false))))
  (:`Completed`
    (if (not (`self.Creating`))
      (`/Engine/EditorBlueprintResources/StandardMacros.IsValid` (`self.WheelRef`)
        (:`Is Valid`
          (switch `int` (`/Game/BattleWizardPBR/WBP_SelectWheel.CurrentSelectionIndex` (`self.WheelRef`))
            (:`0`
              (`Widget.RemoveFromParent` (`self.WheelRef`))
              (set `self.CanMove` true)
              (set `self.Destroying` false)
              (set `/Game/BattleWizardPBR/Animations/ABP_Wizard.Action` "NewEnumerator0" (`self.ActionBPRef`)))
            (:`1`
              (`Widget.RemoveFromParent` (`self.WheelRef`))
              (set `self.CanMove` true)
              (if (>= (`self.Energy`) 20)
                (bind _returnvalue_3 (`GridManager.GetAllTilesOfState` (`self.GridManager`) "Selected"))
                (if (not (`KismetArrayLibrary.Array_IsEmpty` _returnvalue_3))
                  (bind _returnvalue_4 (`GridManager.GetTileData` (`self.GridManager`) (`|GetArrayItem` _returnvalue_3)))
                  (set `/Game/LevelPrototyping/BP_LevelGlobals.DestroyPhase` true (`self.GlobalVar`))
                  (`ExponentialHeightFogComponent.SetSkyAtmosphereAmbientContributionColorScale` (`ExponentialHeightFog.Component` (`self.FogRef`)) (struct :`R` 0.768151 :`G` 0.401978 :`B` 1.0 :`A` 1.0))
                  (bind (_index _gcost _hcost _fcost _movementcost _parentindex _neighbors _tiletransform _tiletype) (break `TileData` _returnvalue_4))
                  (switch `name` _tiletype
                    (:`Ground`
                      (`GridManager.SetTileType` _gridmanager _index "Pit" "Runtime" true)
                      (bind _returnvalue_5 (`KismetMathLibrary.Equal_IntPointIntPoint` _index (`/Game/Werewolf/BP_Werewolf.Current Cord` (`self.WerewolfRef`))))
                      (if _returnvalue_5
                        (set `/Game/Werewolf/BP_Werewolf.StunCountdown` 2 _werewolfref)
                        (set `/Game/Werewolf/Animation/ABP_Werewolf.Stunned` true _actionbpref)))
                    (:`Tree`
                      (`GridManager.SetTileType` _gridmanager _index "Ground" "Runtime" true))
                    (:`Bridge`
                      (`GridManager.SetTileType` _gridmanager _index "Water" "Runtime" true)
                      (if _returnvalue_5
                        (set `/Game/Werewolf/BP_Werewolf.StunCountdown` 3 _werewolfref)
                        (set `/Game/Werewolf/Animation/ABP_Werewolf.Stunned` true _actionbpref))))
                  (set `self.Energy` (- (`self.Energy`) 20))
                  (`/Game/LevelPrototyping/BP_LevelGlobals.AdvanceTurn` (`self.GlobalVar`))
                  (set `self.Destroying` false)
                  (set `/Game/BattleWizardPBR/Animations/ABP_Wizard.Action` "NewEnumerator0" (`self.ActionBPRef`)))))))))))

(fn `ContainsPoint`
  (returns (Contains :type Boolean))
  (locals (TileFound :type Boolean))
  (set `local.TileFound` false)
  (for _array_element (`self.TilesNearWizard`)
    (set `local.TileFound` (or (`KismetMathLibrary.Equal_IntPointIntPoint` _array_element (`self.CurrentTile`)) (`local.TileFound`))))
  (return (`local.TileFound`)))

(fn `RotateToTarget`
  (params (`Target location` :type "IntPoint Structure"))
  (bind (_x _y) (break `IntPoint` `Target location`))
  (bind (_x_2 _y_2) (break `IntPoint` (`self.CurrentCord`)))
  (bind _returnvalue (- _x _x_2))
  (`self.K2_SetActorRotation` (`KismetMathLibrary.MakeRotator` 0.0 0.0 (`KismetMathLibrary.SelectFloat` (`KismetMathLibrary.SelectFloat` 0.0 180.0 (== _returnvalue 1)) (`KismetMathLibrary.SelectFloat` 90.0 -90.0 (== (- _y _y_2) 1)) (!= _returnvalue 0)))))

(fn `SelectTileNearWizard`
  (bind _returnvalue (`GridUtils.GetTileUnderCursor` (`GameplayStatics.GetPlayerController` 0)))
  ;[0 0 0] This function highlights the tile under cursor.
  (if (`KismetMathLibrary.BooleanNOR` (`self.Creating`) (`self.Destroying`))
    ;;[0 0 0] Check if we're hovering over a new tile
    (if (not (`KismetMathLibrary.Equal_IntPointIntPoint` _returnvalue (`self.HoveredTile`)))
      (set `self.CurrentTile` _returnvalue)
      ;;[0 0 0] ScopeLock may not be needed
      ;; if you only use static pathfinding.
      ;; (Saves performance)
      (`GridManager.RemoveStateFromTile` (`self.GridManager`) (`self.HoveredTile`) "Selected" true true)
      ;;[0 0 0] Check if the new tile is within grid boundary
      (bind _returnvalue_2 (`GridUtils.IsTileWithinBounds` (`self.CurrentTile`) (`GridUtils.GetIsHex`)))
      (if _returnvalue_2
        ;; Check if hovered tile is near wizard
        (bind _contains (`self.ContainsPoint`))
        (if _contains
          ;;[0 0 0] ScopeLock may not be needed
          ;; if you only use static pathfinding.
          ;; (Saves performance)
          (`GridManager.AddStateToTile` (`self.GridManager`) (`self.CurrentTile`) "Selected" true true)
          (set `self.HoveredTile` (`self.CurrentTile`)))))))

(fn `UpdateTilesNearWizard`
  (bind _currentcord (`self.CurrentCord`))
  (set `self.TilesNearWizard` (`|MakeArray` (+ _currentcord (`KismetMathLibrary.Conv_Vector2DToIntPoint` (`KismetMathLibrary.MakeVector2D` 0.0 -1.0))) (+ _currentcord (`KismetMathLibrary.Conv_Vector2DToIntPoint` (`KismetMathLibrary.MakeVector2D` 0.0 1.0))) (+ _currentcord (`KismetMathLibrary.Conv_Vector2DToIntPoint` (`KismetMathLibrary.MakeVector2D` 1.0))) (+ _currentcord (`KismetMathLibrary.Conv_Vector2DToIntPoint` (`KismetMathLibrary.MakeVector2D` -1.0))))))

(fn `UserConstructionScript`
  (`SceneComponent.K2_AttachToComponent` (`self.Staff03SM`) (`self.Mesh`) "RightHandSocket" "SnapToTarget" "SnapToTarget" "SnapToTarget" false))